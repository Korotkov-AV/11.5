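; GM_pro3 is a game mode that runs a match countdown and returns the game to a menu level when time runs out.
; On BeginPlay it starts a looping one-second timer whose event decrements GameTime.
; When GameTime reaches zero, it clears the timer and opens the Menu level.
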(event Custom|CustomEvent
  (bind _output_get (Variables|Default|SetGameTime (- (Variables|Default|GetGameTime) 1)))
  (if (== _output_get 0)
    (Utilities|Time|ClearandInvalidateTimerbyHandle (Variables|Default|GetGameTimerHandle))
    (Game|OpenLevel(byObjectReference) "/Game/pro3/levels/menu.menu")))

(event EventBeginPlay
  (bind _returnvalue (Utilities|Time|SetTimerbyEvent (delegate Custom|CustomEvent) 1.0 true))
  (Variables|Default|SetGameTimerHandle _returnvalue))

(event EventTick
  (params (DeltaSeconds :type Float%20%28single-precision%29)))

(fn ConstructionScript)